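; CameraPawnBP is a camera pawn for mouse edge scrolling, with the cursor shown on BeginPlay.
; Each Tick it divides the mouse position by the viewport size, corrected for viewport scale, and compares it to MoveCamBorderPercentage on both axes.
; The right edge calls MoveRight with CamMaxMoveSpeed and delta time.
; The left, top and bottom edges only print debug strings so far.
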(event `self.ReceiveBeginPlay`
  (set `PlayerController.bShowMouseCursor` true (`GameplayStatics.GetPlayerController` 0)))

(event `self.ReceiveTick`
  (params (DeltaSeconds :type "Float (single-precision)"))
  (bind (_returnvalue_x _returnvalue_y) (`KismetMathLibrary.BreakVector2D` (`WidgetLayoutLibrary.GetViewportSize`)))
  (bind _returnvalue (`WidgetLayoutLibrary.GetViewportScale`))
  (bind _movecamborderpercentage (`self.MoveCamBorderPercentage`))
  (bind _returnvalue_2 (- 1.0 _movecamborderpercentage))
  (bind _returnvalue_3 (`WidgetLayoutLibrary.GetMousePositionOnViewport`))
  (bind _returnvalue_4 (/ (`KismetMathLibrary.BreakVector2D` _returnvalue_3) (/ _returnvalue_x _returnvalue)))
  (if (>= _returnvalue_4 _returnvalue_2)
    (`self.MoveRight` (`self.CamMaxMoveSpeed`) DeltaSeconds)
    (elif (<= _returnvalue_4 _movecamborderpercentage)
      (`KismetSystemLibrary.PrintString` "left")))
  (bind _returnvalue_5 (/ (`.Y` (`KismetMathLibrary.BreakVector2D` _returnvalue_3)) (/ _returnvalue_y _returnvalue)))
  (if (>= _returnvalue_5 _returnvalue_2)
    (`KismetSystemLibrary.PrintString` "down")
    (elif (<= _returnvalue_5 _movecamborderpercentage)
      (`KismetSystemLibrary.PrintString` "up"))))

(fn `UserConstructionScript`)